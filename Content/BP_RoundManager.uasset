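; Round manager meant to spawn random batches of AI mobs at randomized intervals, though that loop is disconnected and Tick does nothing.
; SpawnMob spawns an AI at a random point in the box spanned by two ZoneA markers.
; It takes pawn class and behavior tree from separate GetRandomMob calls.
; GetRandomMob's graph holds only an unused random pick between BP_MobB and BP_MobScareCrow.
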(event EventTick
  (params (DeltaSeconds :type Float%20%28single-precision%29)))

(fn ConstructionScript)

(fn SpawnMob
  (bind (_pawn _behaviortree) (Utilities|GetRandomMob))
  (bind _vector (CallFunction|RandomVectorZoneA))
  (AI|SpawnAIFromClass _pawn _behaviortree _vector "0, 0, 0" false 0))

(fn RandomVectorZoneA
  (bind _zoneamarkers (Variables|Markers|GetZoneAMarkers))
  (bind _output (Utilities|Array|Get(acopy) _zoneamarkers))
  (bind _output_2 (Utilities|Array|Get(acopy) _zoneamarkers 1))
  (bind _returnvalue (Transformation|GetActorLocation _output))
  (bind _returnvalue_2 (Transformation|GetActorLocation _output_2))
  (return (Math|Vector|MakeVector (Math|Random|RandomFloatinRange (Math|Float|Min(Float) (.x _returnvalue) (.x _returnvalue_2)) (Math|Float|Max(Float) (.x _returnvalue) (.x _returnvalue_2))) (Math|Random|RandomFloatinRange (Math|Float|Min(Float) (.y _returnvalue) (.y _returnvalue_2)) (Math|Float|Max(Float) (.y _returnvalue) (.y _returnvalue_2))) (Math|Random|RandomFloatinRange (Math|Float|Min(Float) (.z _returnvalue) (.z _returnvalue_2)) (Math|Float|Max(Float) (.z _returnvalue) (.z _returnvalue_2))))))