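; Parent Blueprint for flying mobs that navigate in 3D with Mercuna.
; Helpers test navigability, clamp pathfinding targets into the nav octree, check height limits, stop movement and destroy the actor.
; ToggleChaseMode switches movement between fast chase and slow speeds, while Tick can lock the mesh to a fixed world rotation via quaternion.
; A delayed check that kills mobs stuck outside navigable space is present but disconnected.
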(event EventTick
  (params (DeltaSeconds :type Float%20%28single-precision%29))
  (Utilities|FlowControl|Sequence
    (:then_0
      (if (Variables|Default|GetbFixRotate)
        (bind _returnvalue (Class|QuaternionLib|EulertoQuaternion (Variables|Default|GetFixRotator)))
        (Class|QuaternionLib|SetWorldRotationQuat (Variables|Character|GetMesh) _returnvalue)))))

(fn ConstructionScript)

(fn IsNavigatable
  (params (Vector :type Vector :default "0, 0, 0"))
  (bind _result (Class|MercunaNavOctree|IsNavigable (Class|Mercuna3DNavigationComponent|GetNavOctree (Variables|Default|GetMercuna3DNavigation)) Vector 0.0))
  (return _result))

(fn PathfindVector
  (bind _returnvalue (Class|FlyingMobParent|PathFind))
  (bind _clampedposition (Class|MercunaNavOctree|ClamptoNavigable (Class|Mercuna3DNavigationComponent|GetNavOctree (Variables|Default|GetMercuna3DNavigation)) _returnvalue 0.0 0.0))
  (return _clampedposition))

(fn ToggleChaseMode
  (params (IsChasePlayer :type Boolean))
  (bind _mercuna3dmovement (Variables|Default|GetMercuna3DMovement))
  (if IsChasePlayer
    (Class|Mercuna3DMovementComponent|SetMovementProperties _mercuna3dmovement (Utilities|Struct|MakeMercuna3DMovementProperties 2.5e+03 (Utilities|Struct|MakeMercuna3DMovementAccelerations 9e+02 9e+02 9e+02) 1.5 1.5 2.5 false "(Upward=300.000000,Downward=300.000000)"))
    (else
      (Class|Mercuna3DMovementComponent|SetMovementProperties _mercuna3dmovement (Utilities|Struct|MakeMercuna3DMovementProperties 2e+02 (Utilities|Struct|MakeMercuna3DMovementAccelerations 3e+02 3e+02 1.5e+02) 1.5 1.5 2.5 false "(Upward=300.000000,Downward=300.000000)")))))

(fn ValidOctreeRange
  (bind _returnvalue (Transformation|GetActorLocation))
  (return (< (.z _returnvalue) (+ (Variables|Default|GetMoveableMinZ) 1e+02)) (> (.z _returnvalue) (- (Variables|Default|GetMoveableMaxZ) 1e+02))))

(fn StopMove
  (Class|Mercuna3DNavigationComponent|Stop (Variables|Default|GetMercuna3DNavigation)))

(fn Die
  (Actor|DestroyActor))