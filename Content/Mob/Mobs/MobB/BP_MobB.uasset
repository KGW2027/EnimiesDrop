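; BP_MobB is a ranged mob using Mercuna 3D navigation, with its stats, AI settings and drops defined in GetMobData.
; Attack cancels movement, spawns a projectile at the mesh's ProjectileFixer socket, passes it to the parent attack, plays a sound and fires toward the target.
; Separate SpawnProjectile and ShootProjectile functions implement a preload-and-detach reload cycle, which Attack bypasses.
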(event EventBeginPlay
  (|CallParentFunction))

(fn ConstructionScript)

(fn SpawnProjectile
  (if (not (Variables|Default|GetbProjectileReloaded))
    (bind _returnvalue (Game|SpawnActorfromClass "/Game/Mob/Projectile/BP_MobB_Projectile.BP_MobB_Projectile_C" (Math|Transform|MakeTransform "0, 0,10000.000000" "0, 0, 0" "1.000000,1.000000,1.000000") "AlwaysSpawn" 0 0))
    (bind _output_get (Variables|Default|SetProjectile _returnvalue))
    (Transformation|AttachComponentToComponent _output_get (Variables|Default|GetMobB-Merge) "ProjectileFixer" "SnapToTarget" "SnapToTarget" "SnapToTarget" true)
    (Variables|Default|SetbProjectileReloaded true)))

(fn ShootProjectile
  (params (LaunchVector :type Vector))
  (bind _projectile (Variables|Default|GetProjectile))
  (if (Variables|Default|GetbProjectileReloaded)
    (Transformation|DetachFromActor _projectile "KeepWorld" "KeepWorld" "KeepWorld")
    (Default|Shoot _projectile LaunchVector)
    (Variables|Default|SetbProjectileReloaded false)))

(fn GetMobData
  (return (Utilities|Struct|MakeMobInfoData (Utilities|Struct|MakeMobDropTable 0 1e+02 1e+01 2e+01) (Utilities|Struct|MakeMobStats "MobB" 5e+01 0.0 0.0) (Utilities|Struct|MakeMobAISettings 9e+02 1.6e+03 1e+03 3e+03 5e+03 2e+03 5.0 1e+03 3.0))))

(fn Attack
  (params (Target :type Actor%20Object%20Reference))
  (bind _returnvalue (Transformation|GetActorLocation))
  (Class|Mercuna3DNavigationComponent|CancelMovement (Variables|Default|GetMercuna3DNavigation))
  (bind _returnvalue_2 (Game|SpawnActorfromClass "/Game/Mob/Projectile/BP_MobB_Projectile.BP_MobB_Projectile_C" (Math|Transform|MakeTransform (Transformation|GetSocketLocation (Variables|Default|GetMobB-Merge) "ProjectileFixer") "0, 0, 0" "1.000000,1.000000,1.000000") "AlwaysSpawn" 0 0))
  (|CallParentFunction _returnvalue_2)
  (Audio|PlaySoundatLocation "/Game/Mob/Mobs/MobB/MobB_Attack_Cue.MobB_Attack_Cue" _returnvalue "0, 0, 0" 1.0 1.0 0.0 "/Game/Mob/Mobs/SA_MobSoundAttenuation.SA_MobSoundAttenuation" "/Game/Audio/SC_SoundConcurrency.SC_SoundConcurrency" 0 0)
  (Default|Shoot _returnvalue_2 (* (Math|Vector|RotateVector "1.000000, 0,0.000000" (Math|Rotator|FindLookatRotation _returnvalue (Transformation|GetActorLocation Target))) 2500))
  (return))