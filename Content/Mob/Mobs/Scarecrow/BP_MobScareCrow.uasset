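; Scarecrow mob Blueprint that takes hits and grants experience on death in an RPG.
; BeginPlay sets its health and drop table.
; Hit plays a punch sound at the mob's location, then passes the damage to the parent implementation.
; MobDead awards the drop table's truncated experience to the Victim argument if it is an RPGCharacter, then always runs the parent death logic.
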(event EventBeginPlay
  (Variables|Default|SetHealth 1e+01)
  (Variables|Default|SetDropTable (Utilities|Struct|MakeMobDropTable 0 5e+01 0.0 0.0)))

(event EventHit
  (params (Victim :type Pawn%20Object%20Reference) (Damage :type Float%20%28single-precision%29))
  (Audio|PlaySoundatLocation "/Game/Audio/Punch_Skin_Cue.Punch_Skin_Cue" (Transformation|GetActorLocation) "0, 0, 0" 1.0 1.0 0.0 0 0 0 0)
  (|CallParentFunction Victim Damage))

(event EventMobDead
  (params (Victim :type Pawn%20Object%20Reference))
  (bind _asrpgcharacter (Utilities|Casting|CastToRPGCharacter Victim)
    (:then
      (Class|RPGCharacter|ExpUp _asrpgcharacter (Math|Float|Truncate (.expdrop (Variables|Default|GetDropTable))))
      (|CallParentFunction Victim))
    (:CastFailed
      (|CallParentFunction Victim))))

(fn ConstructionScript)