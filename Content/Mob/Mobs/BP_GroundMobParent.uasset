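; Parent Blueprint for ground-based mobs that navigate with Mercuna ground navigation.
; On BeginPlay it runs the parent logic and binds its skeletal mesh to a Niagara system user variable.
; Tick destroys the mob once it falls below a Z threshold, and InitNavComponent returns the MercunaGroundNavigation component.
; ChangeRotate is an empty function here.
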(event EventBeginPlay
  (|CallParentFunction)
  (Class|NiagaraFunctionLibrary|OverrideSystemUserVariableSkeletalMeshComponent (Variables|Default|GetNiagaraSystem) "MobSkeletalMesh" (Variables|Character|GetMesh)))

(event Collision|EventActorBeginOverlap
  (params (OtherActor :type Actor%20Object%20Reference)))

(event EventTick
  (params (DeltaSeconds :type Float%20%28single-precision%29))
  (if (<= (.z (Transformation|GetActorLocation)) -1e+03)
    (Actor|DestroyActor)))

(fn ConstructionScript)

(fn ChangeRotate
  (params (TargetRotate :type Rotator)))

(fn InitNavComponent
  (return (Variables|Default|GetMercunaGroundNavigation)))