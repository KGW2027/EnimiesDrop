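; BP_MobB is a mob Blueprint that starts with 50 health and fires BP_MobB_Projectile.
; SpawnProjectile spawns a projectile high above the origin when none is loaded, then snaps it to the ProjectileFixer socket on MobBMerge.
; ShootProjectile detaches the loaded projectile in world space and calls its Shoot with a launch vector.
; The ProjectileReloaded flag keeps one projectile loaded at a time and blocks firing when none is ready.
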(event EventBeginPlay
  (Variables|Default|SetHealth 5e+01))

(fn ConstructionScript)

(fn SpawnProjectile
  (if (not (Variables|Default|GetbProjectileReloaded))
    (bind _returnvalue (Game|SpawnActorfromClass "/Game/Mob/Projectile/BP_MobB_Projectile.BP_MobB_Projectile_C" (Math|Transform|MakeTransform "0, 0,10000.000000" "0, 0, 0" "1.000000,1.000000,1.000000") "AlwaysSpawn" 0 0))
    (bind _output_get (Variables|Default|SetProjectile _returnvalue))
    (Transformation|AttachComponentToComponent _output_get (Variables|Default|GetMobB-Merge) "ProjectileFixer" "SnapToTarget" "SnapToTarget" "SnapToTarget" true)
    (Variables|Default|SetbProjectileReloaded true)))

(fn ShootProjectile
  (params (LaunchVector :type Vector))
  (bind _projectile (Variables|Default|GetProjectile))
  (if (Variables|Default|GetbProjectileReloaded)
    (Transformation|DetachFromActor _projectile "KeepWorld" "KeepWorld" "KeepWorld")
    (Default|Shoot _projectile LaunchVector)
    (Variables|Default|SetbProjectileReloaded false)))